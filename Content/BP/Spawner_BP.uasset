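; Spawner actor that periodically spawns AI pawns while the player character is inside its collision sphere.
; Sphere overlap events for MyTestCharacter_BP toggle an in-range flag and print debug messages.
; While the flag is set, Tick runs a random-length Delay, then spawns Enemy, Peasant or an unset third class option, chosen at random, at the Arrow component's transform.
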(event OnComponentBeginOverlap(CollisionSphere)
  (params (OverlappedComponent :type Primitive%20Component%20Object%20Reference) (OtherActor :type Actor%20Object%20Reference) (OtherComp :type Primitive%20Component%20Object%20Reference) (OtherBodyIndex :type Integer) (bFromSweep :type Boolean) (SweepResult :type Hit%20Result%20Structure%20%28by%20ref%29))
  (Utilities|Casting|CastToMyTestCharacter_BP OtherActor)
  (Development|PrintString "Player in" true true "(R=1.000000,G=0.032703,B=0.092427,A=1.000000)")
  (Variables|Default|SetIsInRange true))

(event OnComponentEndOverlap(CollisionSphere)
  (params (OverlappedComponent :type Primitive%20Component%20Object%20Reference) (OtherActor :type Actor%20Object%20Reference) (OtherComp :type Primitive%20Component%20Object%20Reference) (OtherBodyIndex :type Integer))
  (Utilities|Casting|CastToMyTestCharacter_BP OtherActor)
  (Development|PrintString "Player out" true true "(R=0.000000,G=0.173611,B=0.000742,A=1.000000)")
  (Variables|Default|SetIsInRange false))

(event EventBeginPlay)

(event Collision|EventActorBeginOverlap
  (params (OtherActor :type Actor%20Object%20Reference)))

(event EventTick
  (params (DeltaSeconds :type Float%20%28single-precision%29))
  (bind _arrow (Variables|Default|GetArrow))
  (if (Variables|Default|GetIsInRange)
    (Utilities|FlowControl|Delay (Math|Random|RandomFloatinRange 2.0 4.0))
    (AI|SpawnAIFromClass (Utilities|Select :Index (Math|Random|RandomIntegerinRange 0 2) :Option%200 (Variables|Default|GetEnemy) :Option%201 (Variables|Default|GetPeasant) :Option%202 0) 0 (Transformation|GetWorldLocation _arrow) (Transformation|GetWorldRotation _arrow) false 0)))

(fn ConstructionScript)